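; GameInstance that wraps PlayFab login and Economy calls for the game's currency, inventory and store.
; Init sets the title ID; login uses a hardcoded test custom ID, creating the account if needed, and opens the main menu on success.
; Filtered inventory queries cache currency or catalog items, while store searches and inventory updates are broadcast through dispatchers.
; Purchases send a price and item to a fixed store, printing the transaction IDs.
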(event Custom|OnFailure_PlayFab
  (params (error :type Play%20Fab%20Error%20Structure) (customData :type Object%20Object%20Reference))
  ;[1 0.1875 0.1875 1 34] ON FAILURE
  (Development|PrintString (Utilities|String|Append (.errorname error) "" (.errordetails error)) true true "(R=0.000000,G=0.660000,B=1.000000,A=1.000000)" 5.0 "1"))

(event Custom|OnPurchase_Success
  (params (result :type Economy%20Purchase%20Inventory%20Items%20Response%20Structure) (customData :type Object%20Object%20Reference))
  ;[0.6729 0.7124 1 1 34] ON PURCHASE STORE ITEM
  (Development|PrintString (.TransactionIds (Utilities|Struct|BreakEconomyPurchaseInventoryItemsResponse result))))

(event Custom|OnLoginWithPlayFab_Success
  (params (result :type Client%20Login%20Result%20Structure) (customData :type Object%20Object%20Reference))
  ;[0.4281 1 0.3462 1 34] ON LOGIN
  (Development|PrintString (Utilities|String|Append " 
 
PlayFab Id: " (.playfabid result)) true false "(R=0.000000,G=0.660000,B=1.000000,A=1.000000)" 5.0 "1"))

(event Custom|OnGetCatalogItems_Success
  (params (result :type Economy%20Get%20Inventory%20Items%20Response%20Structure) (customData :type Object%20Object%20Reference))
  ;[1 0.8048 0.2192 1 34] SET CURRENCY AND INVENTORY
  (bind _output_get (Variables|Default|SetInventoryItems (.Items (Utilities|Struct|BreakEconomyGetInventoryItemsResponse result))))
  (Default|CallInventoryUpdated _output_get))

(event Custom|OnSearchItems_Success
  (params (result :type Economy%20Search%20Items%20Response%20Structure) (customData :type Object%20Object%20Reference))
  ;[0.7676 0.1536 1 1 34] UPDATE STORE
  (Default|CallStoreUpdated (.Items (Utilities|Struct|BreakEconomySearchItemsResponse result))))

(event Custom|OnGetItems_Success
  (params (result :type Economy%20Get%20Inventory%20Items%20Response%20Structure) (customData :type Object%20Object%20Reference))
  (bind _items (Utilities|Struct|BreakEconomyGetInventoryItemsResponse result))
  (bind _output (Utilities|Array|Get(acopy) _items))
  ;[1 0.8048 0.2192 1 34] SET CURRENCY AND INVENTORY
  (Utilities|IsValid _output
    (:Is%20Valid
      (Variables|Default|SetCurrencyAmount (Class|PlayFabJsonObject|GetNumberField _output "Amount")))))

(event EventPurchaseItem
  (params (IdCurrency :type String) (AmountCurrency :type String) (IdItem :type String))
  ;[0.6729 0.7124 1 1 34] ON PURCHASE STORE ITEM
  (Variables|Default|SetPurchaseItemObject (Class|PlayFabJsonObject|ConstructJsonObject))
  (Variables|Default|SetCurrencyItemObject (Class|PlayFabJsonObject|ConstructJsonObject))
  (Class|PlayFabJsonObject|SetStringField (Variables|Default|GetPurchaseItemObject) "Id" IdItem)
  (Class|PlayFabJsonObject|SetStringField (Variables|Default|GetCurrencyItemObject) "ItemId" IdCurrency)
  (Class|PlayFabJsonObject|SetStringField (Variables|Default|GetCurrencyItemObject) "Amount" AmountCurrency)
  (|PurchaseInventoryItems (Utilities|Struct|MakeEconomyPurchaseInventoryItemsRequest 1 "" 0 false 0 0 "" "" (Variables|Default|GetPurchaseItemObject) 0 (Utilities|Array|MakeArray (Variables|Default|GetCurrencyItemObject)) "1985149a-b936-4664-a73d-a024636f9d14") (delegate Custom|OnPurchase_Success) (EventDispatchers|CreateEvent :!event Custom|OnFailure_PlayFab)))

(event EventInit
  ;[0.1287 0.5964 1] PLAYFAB INITIALIZE
  (Class|PlayFabUtilities|SetPlayFabSettings "763ED"))

(event EventOnLoginPlayFab
  ;[0.4281 1 0.3462 1 34] ON LOGIN
  (bind _successful (|LoginwithCustomID (Utilities|Struct|MakeClientLoginWithCustomIDRequest true "TestAccount") (delegate Custom|OnLoginWithPlayFab_Success) (EventDispatchers|CreateEvent :!event OnFailurePlayfab))
    (:OnPlayFabResponse
      (if _successful
        (Game|OpenLevel(byObjectReference) "/Game/Maps/MainMenu.MainMenu")))))

(event EventSetCurrencyandInventoryPlayFab
  (params (bHasToUpdateCurrency :type Boolean))
  ;[1 0.8048 0.2192 1 34] SET CURRENCY AND INVENTORY
  (if bHasToUpdateCurrency
    (bind _output_get (Variables|Default|SetItemSearchType "'currency'"))
    (|GetInventoryItems (Utilities|Struct|MakeEconomyGetInventoryItemsRequest "" "" 10 0 0 (Utilities|String|Append "type eq " _output_get)) (delegate Custom|OnGetItems_Success) (EventDispatchers|CreateEvent :!event Custom|OnFailure_PlayFab))
    (else
      (bind _output_get_2 (Variables|Default|SetItemSearchType "'catalogItem'"))
      (|GetInventoryItems (Utilities|Struct|MakeEconomyGetInventoryItemsRequest "" "" 10 0 0 (Utilities|String|Append "type eq " _output_get_2)) (delegate Custom|OnGetCatalogItems_Success) (EventDispatchers|CreateEvent :!event Custom|OnFailure_PlayFab)))))

(event EventGetStoreItems
  ;[0.7676 0.1536 1 1 34] UPDATE STORE
  (bind _output_get (Variables|Default|SetStore (Class|PlayFabJsonObject|ConstructJsonObject)))
  (Class|PlayFabJsonObject|SetStringField _output_get "Id" "1985149a-b936-4664-a73d-a024636f9d14")
  (|SearchItems (Utilities|Struct|MakeEconomySearchItemsRequest "" 30 0 0 "" "" "" "" "" (Variables|Default|GetStore)) (delegate Custom|OnSearchItems_Success) (EventDispatchers|CreateEvent :!event Custom|OnFailure_PlayFab)))

(fn GetCurrencyandInventoryPlayFab
  (return (Variables|Default|GetCurrencyAmount) (Variables|Default|GetInventory)))